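; A player-controlled flying pawn that moves constantly along its forward vector and fires rockets.
; Pitch and Roll axes apply frame-time-scaled local rotation, while Tick adds forward movement input and Fire spawns a rocket at the actor's transform.
; A RotatingPropeliar function, not called in these graphs, shifts a given component along local X rather than rotating it, reusing the rotation speed variable that drives steering.
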(event EventTick
  (params (DeltaSeconds :type Float%20%28single-precision%29))
  (Pawn|Input|AddMovementInput (Transformation|GetActorForwardVector) 1.0 false))

(event Input|ActionEvents|InputActionFire
  (params (Key :type Key%20Structure :default "None"))
  (:Pressed
    (Game|SpawnActorfromClass "/Game/Blueprints/_Rocket._Rocket_C" (Transformation|GetActorTransform) "AlwaysSpawn" "MultiplyWithRoot" 0 0)))

(event Input|AxisEvents|InputAxisPitch
  (params (AxisValue :type Float%20%28single-precision%29))
  (Transformation|AddActorLocalRotation (Math|Rotator|MakeRotator 0.0 (* AxisValue (Variables|Default|GetPropeliarRotationSpeed) (Utilities|Time|GetWorldDeltaSeconds)) 0.0) false false))

(event Input|AxisEvents|InputAxisRoll
  (params (AxisValue :type Float%20%28single-precision%29))
  (Transformation|AddActorLocalRotation (Math|Rotator|MakeRotator (* AxisValue (Variables|Default|GetPropeliarRotationSpeed) (Utilities|Time|GetWorldDeltaSeconds)) 0.0 0.0) false false))

(fn ConstructionScript)

(fn RotatingPropeliar
  (params (Where :type Scene%20Capture%20Component%20Cube%20Object%20Reference))
  (Transformation|AddLocalOffset Where (Math|Vector|MakeVector (* (Variables|Default|GetPropeliarRotationSpeed) (Utilities|Time|GetWorldDeltaSeconds)) 0.0 0.0) false false))