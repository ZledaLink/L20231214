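; BP_P38 is a P-38 aircraft Blueprint with spinning left and right propellers.
; On BeginPlay it registers the Left and Right components with its BPRotateSceneComponents component, which by its name handles their rotation.
; A RotatePropeller function can roll a given component at PropellerRotationSpeed scaled by delta time, but nothing in these graphs calls it.
; The construction script and NewFunction are empty.
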(event EventBeginPlay
  (Utilities|Array|Add (Variables|/Game/Blueprints/BP_RotateSceneComponents.BP_RotateSceneComponents_C|GetSceneComponents (Variables|Default|GetBP_RotateSceneComponents)) (Variables|Default|GetLeft))
  (Utilities|Array|Add (Variables|/Game/Blueprints/BP_RotateSceneComponents.BP_RotateSceneComponents_C|GetSceneComponents (Variables|Default|GetBP_RotateSceneComponents)) (Variables|Default|GetRight)))

(fn ConstructionScript)

(fn NewFunction)

(fn RotatePropeller
  (params (Where :type Scene%20Component%20Object%20Reference))
  (Transformation|AddLocalRotation Where (Math|Rotator|MakeRotator (* (Utilities|Time|GetWorldDeltaSeconds) (Variables|Speed|GetPropellerRotationSpeed)) 0.0 0.0) false false))